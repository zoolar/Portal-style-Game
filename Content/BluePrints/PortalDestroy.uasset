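; PortalDestroy is an actor, treated as a wall, that removes a portal when a portal projectile hits it.
; Its Hit event checks whether the other actor's class derives from Red_Projectile or, failing that, Blue_projectile.
; It then finds all Red_Portal or Blue_Portal actors to match and destroys the first one, without checking that any exists.
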(event Collision|EventHit
  (params (MyComp :type Primitive%20Component%20Object%20Reference) (Other :type Actor%20Object%20Reference) (OtherComp :type Primitive%20Component%20Object%20Reference) (bSelfMoved :type Boolean) (HitLocation :type Vector :default "0, 0, 0") (HitNormal :type Vector :default "0, 0, 0") (NormalImpulse :type Vector :default "0, 0, 0") (Hit :type Hit%20Result%20Structure%20%28by%20ref%29))
  (bind _returnvalue (Utilities|GetClass Other))
  ;[1 1 1] Checks if projectile hits wall
  (if (Utilities|ClassIsChildOf _returnvalue "/Game/Portal_Gun/Red_Projectile.Red_Projectile_C")
    ;[1 1 1] If projectile hits wall > destroy portal
    (bind _outactors (Actor|GetAllActorsOfClass "/Game/Portal_Gun/Red_Portal.Red_Portal_C"))
    (Actor|DestroyActor (Utilities|Array|Get(acopy) _outactors))
    (elif (Utilities|ClassIsChildOf _returnvalue "/Game/Portal_Gun/Blue_projectile.Blue_projectile_C")
      (bind _outactors_2 (Actor|GetAllActorsOfClass "/Game/Portal_Gun/Blue_Portal.Blue_Portal_C"))
      (Actor|DestroyActor (Utilities|Array|Get(acopy) _outactors_2)))))

(fn ConstructionScript)