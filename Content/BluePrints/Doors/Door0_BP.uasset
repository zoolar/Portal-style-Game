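; Door0_BP is a sliding double-door Blueprint whose two leaves open and close through custom events.
; OpenEvent plays a timeline whose Movement value scales MoveAmount, offsetting DoorL and DoorR in opposite directions from their stored LeftPos and RightPos.
; CloseEvent reverses the same timeline to slide both leaves back.
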(event Custom|OpenEvent
  (bind _movement (Timeline|Timeline_1 Play)
    (:Update
      (Variables|Default|SetMovement _movement)
      (Transformation|SetRelativeLocation (Variables|Default|GetDoor_L) (+ (* (Variables|Default|GetMoveAmount) _movement) (Variables|Default|GetLeftPos)) false false)
      (Transformation|SetRelativeLocation (Variables|Default|GetDoor_R) (- (Variables|Default|GetRightPos) (* (Variables|Default|GetMoveAmount) _movement)) false false))))

(event Custom|CloseEvent
  (bind _movement (Timeline|Timeline_1 Reverse)
    (:Update
      (Variables|Default|SetMovement _movement)
      (Transformation|SetRelativeLocation (Variables|Default|GetDoor_L) (+ (* (Variables|Default|GetMoveAmount) _movement) (Variables|Default|GetLeftPos)) false false)
      (Transformation|SetRelativeLocation (Variables|Default|GetDoor_R) (- (Variables|Default|GetRightPos) (* (Variables|Default|GetMoveAmount) _movement)) false false))))

(fn ConstructionScript)