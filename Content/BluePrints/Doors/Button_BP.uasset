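; Button_BP is a pressure-style button that opens a linked door while something overlaps it.
; Begin and end overlap on the Button component call OpenEvent and CloseEvent on LinkedDoor through the IDoor interface, after checking that it implements it.
; Each call also plays an open or close sound at the world origin rather than at the button.
; Overlaps are neither filtered by actor nor counted, so any end overlap closes the door.
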(event OnComponentBeginOverlap(Button)
  (params (OverlappedComponent :type Primitive%20Component%20Object%20Reference) (OtherActor :type Actor%20Object%20Reference) (OtherComp :type Primitive%20Component%20Object%20Reference) (OtherBodyIndex :type Integer) (bFromSweep :type Boolean) (SweepResult :type Hit%20Result%20Structure%20%28by%20ref%29))
  (bind _linkeddoor (Variables|Default|GetLinkedDoor))
  ;[1 1 1] Open/Close Door
  (if (Utilities|DoesObjectImplementInterface _linkeddoor "/Game/BluePrints/Doors/IDoor.IDoor_C")
    (Default|OpenEvent _linkeddoor)
    (Audio|PlaySoundatLocation "/Game/door_open.door_open" "0, 0, 0")))

(event OnComponentEndOverlap(Button)
  (params (OverlappedComponent :type Primitive%20Component%20Object%20Reference) (OtherActor :type Actor%20Object%20Reference) (OtherComp :type Primitive%20Component%20Object%20Reference) (OtherBodyIndex :type Integer))
  (bind _linkeddoor (Variables|Default|GetLinkedDoor))
  ;[1 1 1] Open/Close Door
  (if (Utilities|DoesObjectImplementInterface _linkeddoor "/Game/BluePrints/Doors/IDoor.IDoor_C")
    (Default|CloseEvent _linkeddoor)
    (Audio|PlaySoundatLocation "/Game/door_close.door_close" "0, 0, 0")))

(fn ConstructionScript)