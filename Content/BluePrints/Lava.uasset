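; Lava hazard actor that drains the first-person character's health and opens the level "Level" once it drops below zero.
; Tick and Hit share one chain that checks whether the Hit event's Other actor is a FirstPersonCharacter.
; Each pass subtracts a small fixed amount from the first character found by GetAllActorsOfClass, not from Other.
; Because Tick reads Other from Hit, damage runs per frame, independent of ongoing contact.
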(event Collision|EventHit
  (params (MyComp :type Primitive%20Component%20Object%20Reference) (Other :type Actor%20Object%20Reference) (OtherComp :type Primitive%20Component%20Object%20Reference) (bSelfMoved :type Boolean) (HitLocation :type Vector :default "0, 0, 0") (HitNormal :type Vector :default "0, 0, 0") (NormalImpulse :type Vector :default "0, 0, 0") (Hit :type Hit%20Result%20Structure%20%28by%20ref%29))
  (if (Utilities|ClassIsChildOf (Utilities|GetClass Other) "/Game/FirstPersonBP/Blueprints/FirstPersonCharacter.FirstPersonCharacter_C")
    (bind _outactors (Actor|GetAllActorsOfClass "/Game/FirstPersonBP/Blueprints/FirstPersonCharacter.FirstPersonCharacter_C"))
    (bind _output_get (Variables|/Game/FirstPersonBP/Blueprints/FirstPersonCharacter.FirstPersonCharacter_C|SetHealth (Utilities|Array|Get(acopy) _outactors) (- (Variables|/Game/FirstPersonBP/Blueprints/FirstPersonCharacter.FirstPersonCharacter_C|GetHealth (Utilities|Array|Get(acopy) _outactors)) 0.1)))
    (Math|Float|CompareFloat _output_get 0.0
      (:<
        (Game|OpenLevel(byName) "Level")))))

(event EventTick
  (params (DeltaSeconds :type Float%20%28single-precision%29))
  (if (Utilities|ClassIsChildOf (Utilities|GetClass (stale Collision|EventHit Other)) "/Game/FirstPersonBP/Blueprints/FirstPersonCharacter.FirstPersonCharacter_C")
    (bind _outactors (Actor|GetAllActorsOfClass "/Game/FirstPersonBP/Blueprints/FirstPersonCharacter.FirstPersonCharacter_C"))
    (bind _output_get (Variables|/Game/FirstPersonBP/Blueprints/FirstPersonCharacter.FirstPersonCharacter_C|SetHealth (Utilities|Array|Get(acopy) _outactors) (- (Variables|/Game/FirstPersonBP/Blueprints/FirstPersonCharacter.FirstPersonCharacter_C|GetHealth (Utilities|Array|Get(acopy) _outactors)) 0.1)))
    (Math|Float|CompareFloat _output_get 0.0
      (:<
        (Game|OpenLevel(byName) "Level")))))

(fn ConstructionScript)